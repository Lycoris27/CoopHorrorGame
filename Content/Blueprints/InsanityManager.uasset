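; InsanityManager Blueprint drives an insanity effect from the distance between two players.
; CalculateInsanityMeter sets InsanityMeter straight to 100 when Player1 and Player2 are farther apart than MaxDistance.
; Above InsanityThreshold, it adds a new post-process component with no settings filled in; the below-threshold check is empty.
; Nothing in the graph calls the event, and BeginPlay is disabled.
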(event `CalculateInsanityMeter`
  ;[1 1 1] Calculates distance between two players
  (if (> (`KismetMathLibrary.Vector_Distance` (`self.K2_GetActorLocation` (`self.Player1`)) (`self.K2_GetActorLocation` (`self.Player2`))) (`self.maxDistance`))
    ;[1 1 1] Checks if insanity meter exceeds threshold
    (bind _output_get (set `self.InsanityMeter` 100.0))
    (if (> _output_get (`self.InsanityThreshold`))
      (bind _returnvalue (`AddComponent|NODE_AddPostProcessComponent-0`))
      (set `PostProcessComponent.Settings` (struct) _returnvalue)
      (if (< (`self.InsanityMeter`) (`self.InsanityThreshold`))
        _))))

(fn `UserConstructionScript`)