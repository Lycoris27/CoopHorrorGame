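; BP_ActivatedPlate is a plate that moves along configured waypoints when activated.
; The construction script copies WayPoints and Duration into an InterpToMovement component and turns off its auto-activation.
; ButtonActivated activates the component and its tick, then waits for Duration before calling ButtonDeactivated, ignoring its Continuous input.
; ButtonDeactivated halts movement by disabling the component's tick, leaving it active.
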(event `ButtonActivated`
  (params (Continuous :type Boolean))
  (bind _interptomovement (`self.InterpToMovement`))
  ;[1 1 1] activates plate
  (`ActorComponent.SetActive` _interptomovement true false)
  (`ActorComponent.SetComponentTickEnabled` _interptomovement true)
  ;[1 1 1] after duration, deactivates its movement
  (`KismetSystemLibrary.Delay` (`self.Duration`))
  (`self.ButtonDeactivated`))

(event `ButtonDeactivated`
  (bind _interptomovement (`self.InterpToMovement`))
  (`ActorComponent.SetActive` _interptomovement true false)
  (`ActorComponent.SetComponentTickEnabled` _interptomovement false))

(fn `UserConstructionScript`
  (bind _interptomovement (`self.InterpToMovement`))
  (set `InterpToMovementComponent.ControlPoints` (`self.WayPoints`) _interptomovement)
  (set `InterpToMovementComponent.Duration` (`self.Duration`) _interptomovement)
  (`ActorComponent.SetAutoActivate` _interptomovement false))