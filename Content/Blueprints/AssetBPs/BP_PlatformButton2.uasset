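; Interactable button Blueprint that triggers timed changes on four linked targets: a platform, a plate, a round-platform blockade and a base platform.
; Interact runs four Sequence branches with parallel Delays driven by Duration.
; The platform gets explicit activate and deactivate calls; plate and base get ButtonActivated at start and end.
; The blockade's first call waits half the Duration, its second another full Duration, despite the comment saying it resets when time ends.
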(event `/Game/Blueprints/Blueprint_Interfaces/InteractInterface.Interact`
  (params (Player :type "/Game/BP_ThirdPersonCharacter Object Reference"))
  (bind _targetplatform (`self.TargetPlatform`))
  (bind _targetplate (`self.TargetPlate`))
  (bind _targetplatformround (`self.TargetPlatformRound`))
  (`|ExecutionSequence`
    (:`then_0`
      ;[1 1 1] The platform is active for a duration, then is deactivated
      (`/Game/Blueprints/AssetBPs/BP_Activatedplatform.ButtonActivated` _targetplatform (`self.IsContinuous`))
      (`KismetSystemLibrary.Delay` (`KismetMathLibrary.Conv_IntToDouble` (`self.Duration`)))
      (`/Game/Blueprints/AssetBPs/BP_Activatedplatform.ButtonDeactivated` _targetplatform))
    (:`then_1`
      ;[1 1 1] The plate is activated, raising it, and then after the duration, it lowers it back down
      (`/Game/Blueprints/AssetBPs/BP_ActivatedPlate.ButtonActivated` _targetplate false)
      (`KismetSystemLibrary.Delay` (`KismetMathLibrary.Conv_IntToDouble` (`self.Duration`)))
      (`/Game/Blueprints/AssetBPs/BP_ActivatedPlate.ButtonActivated` _targetplate false))
    (:`then_2`
      ;[1 1 1] When half of the time limit remains, the blockade is removed, when the duration ends, the blockade is placed back again
      (`KismetSystemLibrary.Delay` (`KismetMathLibrary.Conv_IntToDouble` (/ (`self.Duration`) 2)))
      (`/Game/Blueprints/AssetBPs/BP_Activatedplatform.ButtonActivated` _targetplatformround false)
      (`KismetSystemLibrary.Delay` (`KismetMathLibrary.Conv_IntToDouble` (`self.Duration`)))
      (`/Game/Blueprints/AssetBPs/BP_Activatedplatform.ButtonActivated` _targetplatformround false))
    (:`then_3`
      ;[1 1 1] Start, release platform, end remove platform
      (`/Game/Blueprints/AssetBPs/BP_Activatedplatform.ButtonActivated` (`self.TargetPlatformBase`) false)
      (`KismetSystemLibrary.Delay` (`KismetMathLibrary.Conv_IntToDouble` (`self.Duration`)))
      (`/Game/Blueprints/AssetBPs/BP_Activatedplatform.ButtonActivated` (`self.TargetPlatformBase`) false))))

(fn `UserConstructionScript`)