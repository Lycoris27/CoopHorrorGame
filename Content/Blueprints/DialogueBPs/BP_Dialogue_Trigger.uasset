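; Dialogue trigger that shows lines from a Dialogue array in a Test_Dialogue widget when an actor implementing BP_Dial enters TriggerZone.
; Each qualifying overlap calls that actor's UpdatePlayersDialogueInfoMessage, but only the first starts Talk, as DialogueOpen is never reset here.
; Each Talk call advances TalkIndex, creating the widget if needed to show that line, or removing it once the array runs out.
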(event `/Game/Blueprints/DialogueBPs/BP_Dial.Talk`
  (if true
    (bind _result (`/Engine/EditorBlueprintResources/StandardMacros.IncrementInt` (`self.talkIndex`))
      (:`  `
        (if (< _result (`KismetArrayLibrary.Array_Length` (`self.dialogue`)))
          (`self.WidgetVariable`
            (:`then`
              _)
            (:`else`
              (bind _returnvalue (`|CreateWidget` "/Game/MitchLevels/Widgets/Test_Dialogue.Test_Dialogue_C" (`GameplayStatics.GetPlayerController` 0)))
              (bind _output_get (set `self.WidgetVariable` _returnvalue))
              (`UserWidget.AddToViewport` _output_get 0)))
          (`TextBlock.SetText` (`/Game/MitchLevels/Widgets/Test_Dialogue.DialogueText` (`self.WidgetVariable`)) (`KismetTextLibrary.Conv_StringToText` (`|GetArrayItem` (`self.dialogue`) (`self.talkIndex`))))
          (else
            (`Widget.RemoveFromParent` (`self.WidgetVariable`))))))))

(event `self.TriggerZone.OnComponentBeginOverlap`
  (params (OverlappedComponent :type "PrimitiveComponent Object Reference") (OtherActor :type "Actor Object Reference") (OtherComp :type "PrimitiveComponent Object Reference") (OtherBodyIndex :type Integer) (bFromSweep :type Boolean) (SweepResult :type "HitResult Structure (by ref)"))
  (if (`KismetSystemLibrary.DoesImplementInterface` OtherActor "/Game/Blueprints/DialogueBPs/BP_Dial.BP_Dial_C")
    (message `/Game/Blueprints/DialogueBPs/BP_Dial.UpdatePlayersDialogueInfo` OtherActor)
    (if (not (`self.DialogueOpen`))
      (set `self.DialogueOpen` true)
      (`/Game/Blueprints/DialogueBPs/BP_Dial.Talk`))))

(fn `UserConstructionScript`)