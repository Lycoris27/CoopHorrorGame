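; BP_Door is a puzzle door actor that opens and closes in response to switch activation and deactivation events.
; SwitchActivated and SwitchDeactivated set the active pressure switch count to one or zero rather than counting, then compare it to the number needed.
; The result plays or reverses the ActivateDoor timeline, whose DoorPosition track drives the Door component's relative Z location.
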(event `SwitchActivated`
  (set `self.PressureSwitchesActive` 1)
  (if (>= (`self.PressureSwitchesActive`) (`self.PressureSwitchesNeeded`))
    (bind (_direction _doorposition) (`Timeline|ActivateDoor` :!label _label)
      (:`Update`
        (`SceneComponent.K2_SetRelativeLocation` (`self.Door`) (`KismetMathLibrary.MakeVector` 0.0 0.0 _doorposition) false false)))
    (else
      (goto _label :!via `Reverse`))))

(event `SwitchDeactivated`
  (set `self.PressureSwitchesActive` 0)
  (if (>= (`self.PressureSwitchesActive`) (`self.PressureSwitchesNeeded`))
    (goto _label)
    (else
      (goto _label :!via `Reverse`))))

(fn `UserConstructionScript`)