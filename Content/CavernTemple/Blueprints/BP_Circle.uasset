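; BP_Circle is a trigger actor in the Cavern Temple that switches a Niagara circle effect and the candles on and off.
; Box overlap enables player input, passes InBox to Lights on all BP_Candles_3 actors, and raises the effect's alpha and spawn rates.
; Leaving the box, BeginPlay and pressing 1 share one reset path that disables input, updates candles and zeroes the effect.
; A timeline exists but never runs.
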(event `self.Box.OnComponentBeginOverlap`
  (params (OverlappedComponent :type "PrimitiveComponent Object Reference") (OtherActor :type "Actor Object Reference") (OtherComp :type "PrimitiveComponent Object Reference") (OtherBodyIndex :type Integer) (bFromSweep :type Boolean) (SweepResult :type "HitResult Structure (by ref)"))
  (bind _niagara (`self.Niagara`))
  (set `self.InBox` true)
  (`self.EnableInput` (`GameplayStatics.GetPlayerController` 0))
  ;[1 1 1] Candles
  (bind _outactors (`GameplayStatics.GetAllActorsOfClass` "/Game/CavernTemple/Blueprints/BP_Candles_3.BP_Candles_3_C"))
  (`/Game/CavernTemple/Blueprints/BP_Candles_3.Lights` _outactors (`self.InBox`))
  ;[1 1 1] Circle
  (`NiagaraComponent.SetNiagaraVariableFloat` _niagara "CircleAlpha" 1.0)
  (`NiagaraComponent.SetNiagaraVariableFloat` _niagara "SpawnRate" 100.0)
  (`NiagaraComponent.SetNiagaraVariableFloat` _niagara "SpawnRateCircle" 2.0))

(event `self.Box.OnComponentEndOverlap`
  (params (OverlappedComponent :type "PrimitiveComponent Object Reference") (OtherActor :type "Actor Object Reference") (OtherComp :type "PrimitiveComponent Object Reference") (OtherBodyIndex :type Integer))
  (bind _niagara (`self.Niagara`))
  (set `self.InBox` false :!label _label)
  (`self.DisableInput` (`GameplayStatics.GetPlayerController` 0))
  ;[1 1 1] Candles
  (bind _outactors (`GameplayStatics.GetAllActorsOfClass` "/Game/CavernTemple/Blueprints/BP_Candles_3.BP_Candles_3_C"))
  (`/Game/CavernTemple/Blueprints/BP_Candles_3.Lights` _outactors (`self.InBox`))
  ;[1 1 1] Circle
  (`NiagaraComponent.SetNiagaraVariableFloat` _niagara "CircleAlpha" 0.0)
  (`NiagaraComponent.SetNiagaraVariableFloat` _niagara "SpawnRate" 0.0)
  (`NiagaraComponent.SetNiagaraVariableFloat` _niagara "SpawnRateCircle" 0.0))

(event `self.ReceiveBeginPlay`
  (goto _label))

(event `Key|One`
  (params (Key :type "Key Structure"))
  (:`Pressed`
    (goto _label)))

(fn `UserConstructionScript`)