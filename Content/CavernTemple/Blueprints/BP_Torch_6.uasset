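; BP_Torch_6 is a torch actor combining a Niagara fire effect with a flickering point light.
; The construction script applies exposed settings to fire spawn rate, radius and sprite size, and to light intensity, temperature, volumetric scattering and shadows.
; Tick randomizes intensity each frame between LightIntensity and that value times Flicker.
; A time-seeded random stream is created beforehand, but the random float call does not use it.
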(event `self.ReceiveBeginPlay`)

(event `self.ReceiveTick`
  (params (DeltaSeconds :type "Float (single-precision)"))
  (bind _seconds (`GameplayStatics.GetAccurateRealTime`))
  (bind _light_intensity (`self.Light Intensity`))
  (`KismetMathLibrary.SetRandomStreamSeed` (`KismetMathLibrary.MakeRandomStream` _seconds) _seconds)
  (`LightComponent.SetIntensity` (`self.PointLight`) (`KismetMathLibrary.RandomFloatInRange` _light_intensity (* _light_intensity (`self.Flicker`)))))

(fn `UserConstructionScript`
  (bind _seconds (`GameplayStatics.GetAccurateRealTime`))
  (bind _light_intensity (`self.Light Intensity`))
  (bind _sprite_size (`self.Sprite Size`))
  (bind _niagara (`self.Niagara`))
  (bind _pointlight (`self.PointLight`))
  (`NiagaraComponent.SetNiagaraVariableFloat` (`self.Niagara`) "SpawnRate" (`self.Spawn Rate`))
  (`NiagaraComponent.SetVariableFloat` _niagara "Sphere Radius" (`self.Fire Radius`))
  (`NiagaraComponent.SetVariableVec2` _niagara "ScaleCurve_Scale Factor" (`KismetMathLibrary.MakeVector2D` _sprite_size _sprite_size))
  (`KismetMathLibrary.SetRandomStreamSeed` (`KismetMathLibrary.MakeRandomStream` _seconds) _seconds)
  (`LightComponent.SetIntensity` (`self.PointLight`) (`KismetMathLibrary.RandomFloatInRange` _light_intensity (* _light_intensity (`self.Flicker`))))
  (`LightComponent.SetVolumetricScatteringIntensity` _pointlight (`self.Volumetric Scattering Intensity`))
  (`LightComponent.SetTemperature` _pointlight (`self.Temperature`))
  (`LightComponentBase.SetCastShadows` _pointlight (`self.Cast Shadows`)))