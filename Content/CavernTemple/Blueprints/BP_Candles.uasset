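; Candle prop for the Cavern Temple with five flame components and a flickering light.
; Every Tick sets a random light intensity between LightIntensity and that value times Flicker.
; A time-seeded random stream is created, but the random call does not draw from it.
; The construction script also sets initial intensity, volumetric scattering, temperature and shadow casting, and passes WindIntensity to the flame materials.
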(event `self.ReceiveTick`
  (params (DeltaSeconds :type "Float (single-precision)"))
  (bind _seconds (`GameplayStatics.GetAccurateRealTime`))
  (bind _light_intensity (`self.Light Intensity`))
  (`KismetMathLibrary.SetRandomStreamSeed` (`KismetMathLibrary.MakeRandomStream` _seconds) _seconds)
  (`LightComponent.SetIntensity` (`self.Light`) (`KismetMathLibrary.RandomFloatInRange` _light_intensity (* _light_intensity (`self.Flicker`)))))

(fn `UserConstructionScript`
  (bind _seconds (`GameplayStatics.GetAccurateRealTime`))
  (bind _light_intensity (`self.Light Intensity`))
  (bind _light (`self.Light`))
  (`KismetMathLibrary.SetRandomStreamSeed` (`KismetMathLibrary.MakeRandomStream` _seconds) _seconds)
  (`LightComponent.SetIntensity` _light (`KismetMathLibrary.RandomFloatInRange` _light_intensity (* _light_intensity (`self.Flicker`))))
  (`LightComponent.SetVolumetricScatteringIntensity` _light (`self.Volumetric Scattering Intensity`))
  (`LightComponent.SetTemperature` _light (`self.Temperature`))
  (`LightComponentBase.SetCastShadows` _light (`self.Cast Shadows`))
  (`MeshComponent.SetScalarParameterValueOnMaterials` (`self.Flame`) "WindIntensity (S)" (`self.WindIntensity`))
  (`MeshComponent.SetScalarParameterValueOnMaterials` (`self.Flame1`) "WindIntensity (S)" (`self.WindIntensity`))
  (`MeshComponent.SetScalarParameterValueOnMaterials` (`self.Flame2`) "WindIntensity (S)" (`self.WindIntensity`))
  (`MeshComponent.SetScalarParameterValueOnMaterials` (`self.Flame3`) "WindIntensity (S)" (`self.WindIntensity`))
  (`MeshComponent.SetScalarParameterValueOnMaterials` (`self.Flame4`) "WindIntensity (S)" (`self.WindIntensity`)))