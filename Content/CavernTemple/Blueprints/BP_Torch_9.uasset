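; BP_Torch_9 is a torch Blueprint that applies flicker and light settings, but targets the first BP_Torch_4 found via GetActorOfClass instead of itself.
; The construction script pushes spawn rate to that actor's Niagara effect and sets its point light's intensity, volumetric scattering, temperature and shadows.
; Tick randomizes intensity between LightIntensity and LightIntensity times Flicker; the time-seeded stream does not feed that random call.
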(event `self.ReceiveTick`
  (params (DeltaSeconds :type "Float (single-precision)"))
  (bind _seconds (`GameplayStatics.GetAccurateRealTime`))
  (bind _light_intensity (`self.Light Intensity`))
  (bind _returnvalue (`GameplayStatics.GetActorOfClass` "/Game/CavernTemple/Blueprints/BP_Torch_4.BP_Torch_4_C"))
  (`KismetMathLibrary.SetRandomStreamSeed` (`KismetMathLibrary.MakeRandomStream` _seconds) _seconds)
  (`LightComponent.SetIntensity` (`/Game/CavernTemple/Blueprints/BP_Torch_4.PointLight` _returnvalue) (`KismetMathLibrary.RandomFloatInRange` _light_intensity (* _light_intensity (`self.Flicker`)))))

(fn `UserConstructionScript`
  (bind _seconds (`GameplayStatics.GetAccurateRealTime`))
  (bind _light_intensity (`self.Light Intensity`))
  (bind _returnvalue (`GameplayStatics.GetActorOfClass` "/Game/CavernTemple/Blueprints/BP_Torch_4.BP_Torch_4_C"))
  (`NiagaraComponent.SetNiagaraVariableFloat` (`/Game/CavernTemple/Blueprints/BP_Torch_4.Niagara` _returnvalue) "SpawnRate" (`self.Spawn Rate`))
  (bind _returnvalue_2 (`GameplayStatics.GetActorOfClass` "/Game/CavernTemple/Blueprints/BP_Torch_4.BP_Torch_4_C"))
  (`KismetMathLibrary.SetRandomStreamSeed` (`KismetMathLibrary.MakeRandomStream` _seconds) _seconds)
  (bind _pointlight (`/Game/CavernTemple/Blueprints/BP_Torch_4.PointLight` _returnvalue_2))
  (`LightComponent.SetIntensity` _pointlight (`KismetMathLibrary.RandomFloatInRange` _light_intensity (* _light_intensity (`self.Flicker`))))
  (`LightComponent.SetVolumetricScatteringIntensity` _pointlight (`self.Volumetric Scattering Intensity`))
  (`LightComponent.SetTemperature` _pointlight (`self.Temperature`))
  (`LightComponentBase.SetCastShadows` _pointlight (`self.Cast Shadows`)))