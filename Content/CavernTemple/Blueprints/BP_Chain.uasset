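; Spline-based chain actor that lays copies of a mesh along its spline at construction time, with no runtime logic.
; The construction script adds a Hierarchical Instanced Static Mesh, taking the instance count from the mesh's Y extent minus DistanceAdjustment and dividing spline length by that for spacing.
; Each instance's Y axis points toward the next sample point, with slight random yaw jitter.
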(fn `UserConstructionScript`
  (bind _spline (`self.Spline`))
  (bind _mesh (`self.Mesh`))
  (bind _returnvalue (`SplineComponent.GetSplineLength` (`self.Spline`)))
  (bind _returnvalue_2 (/ _returnvalue (- (.y (`.BoxExtent` (`KismetMathLibrary.BreakBoxSphereBounds` (`StaticMesh.GetBounds` _mesh)))) (`self.Distance Adjustment`))))
  (bind _returnvalue_3 (`KismetMathLibrary.FTrunc` _returnvalue_2))
  (bind _returnvalue_4 (`AddComponent|NODE_AddHierarchicalInstancedStaticMeshComponent-0`))
  (`StaticMeshComponent.SetStaticMesh` _returnvalue_4 _mesh)
  (for _index (range (+ (`KismetMathLibrary.FTrunc` (/ _returnvalue _returnvalue_2)) 1))
    (bind _returnvalue_5 (`SplineComponent.GetLocationAtDistanceAlongSpline` _spline (`KismetMathLibrary.Conv_IntToDouble` (* _index _returnvalue_3)) "Local"))
    (bind (_returnvalue_roll _returnvalue_pitch _returnvalue_yaw) (`KismetMathLibrary.BreakRotator` (`KismetMathLibrary.MakeRotFromY` (- (`SplineComponent.GetLocationAtDistanceAlongSpline` _spline (`KismetMathLibrary.Conv_IntToDouble` (* (+ _index 1) _returnvalue_3)) "Local") _returnvalue_5))))
    (`InstancedStaticMeshComponent.AddInstance` _returnvalue_4 (`KismetMathLibrary.MakeTransform` _returnvalue_5 (`KismetMathLibrary.MakeRotator` _returnvalue_roll _returnvalue_pitch (+ _returnvalue_yaw (`KismetMathLibrary.RandomFloatInRange` -5.0 5.0)))))))